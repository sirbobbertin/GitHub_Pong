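; BP_AI is a computer-controlled mover that follows BP_Ball along the Y axis within fixed bounds.
; Each Tick looks up the ball, stores its position, and SetDirection compares Y values to choose the movement sign.
; The capsule then moves by a fixed MySpeed step per frame, without delta-time scaling or sweep, and snaps back inside when it leaves the hard-coded limits.
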(event EventBeginPlay)

(event Collision|EventActorBeginOverlap
  (params (OtherActor :type Actor%20Object%20Reference)))

(event EventTick
  (params (DeltaSeconds :type Float%20%28single-precision%29))
  (bind _capsulecomponent (Variables|Collision|GetCapsuleComponent))
  (bind _capsulecomponent_2 (Variables|Collision|GetCapsuleComponent))
  (bind _returnvalue (Transformation|GetWorldLocation _capsulecomponent_2))
  (bind _returnvalue_2 (Transformation|GetWorldLocation _capsulecomponent))
  (bind (_x _y _z) (Math|Vector|BreakVector _returnvalue))
  (bind (_x_2 _y_2 _z_2) (Math|Vector|BreakVector _returnvalue_2))
  (bind _returnvalue_3 (Actor|GetActorOfClass "/Game/BP_Ball.BP_Ball_C"))
  (Variables|Default|SetTargetPosition (Transformation|GetActorLocation _returnvalue_3))
  (CallFunction|SetDirection)
  (if (<= _y_2 8e+01)
    (if (<= -8e+02 _y)
      (Transformation|AddLocalOffset (Variables|Collision|GetCapsuleComponent) (Math|Vector|MakeVector 0.0 (* (Variables|Default|GetMoveDir) (Variables|Default|GetmySpeed)) 0.0) false false)
      (else
        (Transformation|SetWorldLocation (Variables|Collision|GetCapsuleComponent) (Math|Vector|MakeVector _x -799.0 _z) false false)))
    (else
      (Transformation|SetWorldLocation (Variables|Collision|GetCapsuleComponent) (Math|Vector|MakeVector _x_2 7e+01 _z_2) false false))))

(event Input|AxisEvents|InputAxisSideMovement
  (params (AxisValue :type Float%20%28single-precision%29)))

(fn ConstructionScript)

(fn SetDirection
  (if (<= (.Y (Math|Vector|BreakVector (Transformation|GetActorLocation))) (.Y (Math|Vector|BreakVector (Variables|Default|GetTargetPosition))))
    (Variables|Default|SetMoveDir 1)
    (elif (>= (.Y (Math|Vector|BreakVector (Transformation|GetActorLocation))) (.Y (Math|Vector|BreakVector (Variables|Default|GetTargetPosition))))
      (Variables|Default|SetMoveDir -1)
      (else
        (Variables|Default|SetMoveDir 0)))))