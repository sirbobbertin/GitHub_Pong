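; BP_Player is a player pawn that slides sideways along the Y axis within fixed bounds.
; Each tick it offsets itself by MoveSpeed times the SideMovement axis, using an unswept local offset rather than movement input.
; When the capsule leaves the allowed Y range, it snaps back to a fixed position at that edge.
; Tick also stores the truncated axis value in MoveDir.
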(event EventBeginPlay)

(event Collision|EventActorBeginOverlap
  (params (OtherActor :type Actor%20Object%20Reference)))

(event EventTick
  (params (DeltaSeconds :type Float%20%28single-precision%29))
  (bind _returnvalue (Input|AxisValues|GetSideMovement))
  (bind _capsulecomponent (Variables|Collision|GetCapsuleComponent))
  (bind _capsulecomponent_2 (Variables|Collision|GetCapsuleComponent))
  (bind _returnvalue_2 (Transformation|GetWorldLocation _capsulecomponent_2))
  (bind _returnvalue_3 (Transformation|GetWorldLocation _capsulecomponent))
  (bind (_x _y _z) (Math|Vector|BreakVector _returnvalue_2))
  (bind (_x_2 _y_2 _z_2) (Math|Vector|BreakVector _returnvalue_3))
  (if (<= -8e+02 _y)
    (if (<= _y_2 1e+02)
      (Transformation|AddActorLocalOffset (Math|Vector|MakeVector 0.0 (* (Variables|Default|GetMoveSpeed) _returnvalue) 0.0) false false)
      (else
        (Transformation|SetWorldLocation (Variables|Collision|GetCapsuleComponent) (Math|Vector|MakeVector _x_2 8e+01 _z_2) false false)))
    (else
      (Transformation|SetWorldLocation (Variables|Collision|GetCapsuleComponent) (Math|Vector|MakeVector _x -789.0 _z) false false)))
  (Variables|Default|SetMoveDir (Math|Float|Truncate _returnvalue)))

(event Input|AxisEvents|InputAxisSideMovement
  (params (AxisValue :type Float%20%28single-precision%29)))

(fn ConstructionScript)