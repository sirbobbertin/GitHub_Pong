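; Pong-style ball that bounces between the player and AI paddles and side walls, driven by ProjectileMovement.
; Overlap casts pick the response: paddles add randomized spin from MoveDir and reverse X with a speed-up, walls add slight jitter and reverse Y.
; Either score zone resets position and velocity without counting points.
; A Tick-fed timer gives both reversals a shared one-second cooldown, though spin applies regardless.
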(event EventBeginPlay)

(event Collision|EventActorBeginOverlap
  (params (OtherActor :type Actor%20Object%20Reference))
  (bind _asbp_player (Utilities|Casting|CastToBP_Player OtherActor)
    (:then
      (CallFunction|HandleBounce (Variables|/Game/BP_Player.BP_Player_C|GetMoveDir _asbp_player)))
    (:CastFailed
      (bind _asbp_ai (Utilities|Casting|CastToBP_AI OtherActor)
        (:then
          (CallFunction|HandleBounce (Variables|/Game/BP_AI.BP_AI_C|GetMoveDir _asbp_ai)))
        (:CastFailed
          (Utilities|Casting|CastToPlayer_ScoreZone OtherActor
            (:then
              (Transformation|SetWorldLocation (Variables|Default|GetDefaultSceneRoot) "0, 0,124.000000" false false :!label _label)
              (Variables|/Script/Engine.MovementComponent|SetVelocity (Variables|Default|GetProjectileMovement) (Math|Vector|MakeVector 2e+02 0.0 0.0)))
            (:CastFailed
              (Utilities|Casting|CastToPlayer_ScoreZone1 OtherActor
                (:then
                  (goto _label))
                (:CastFailed
                  (Utilities|Casting|CastToL_Wall OtherActor
                    (:then
                      _)
                    (:CastFailed
                      (Utilities|Casting|CastToR_Wall OtherActor)))
                  (CallFunction|WallBounce))))))))))

(event EventTick
  (params (DeltaSeconds :type Float%20%28single-precision%29))
  (Variables|Default|SetTimeinReverse (+ DeltaSeconds (Variables|Default|GetTimeinReverse))))

(fn ConstructionScript)

(fn OutOfBounds)

(fn HandleBounce
  (params (Selection :type Integer))
  (bind _returnvalue (Math|Random|RandomFloatinRange -5e+01 5e+01))
  (switch int Selection
    (:-1
      (CallFunction|AddSpin (+ _returnvalue 125.0)))
    (:0
      (CallFunction|AddSpin (Math|Random|RandomFloatinRange -15.0 15.0)))
    (:1
      (CallFunction|AddSpin (+ _returnvalue -125.0))))
  (CallFunction|RevsereX))

(fn AddSpin
  (params (Spin :type Float%20%28single-precision%29))
  (Variables|/Script/Engine.MovementComponent|SetVelocity (Variables|Default|GetProjectileMovement) (+ (Math|Vector|MakeVector 0.0 Spin 0.0) (Variables|/Script/Engine.MovementComponent|GetVelocity (Variables|Default|GetProjectileMovement)))))

(fn RevsereX
  (if (>= (Variables|Default|GetTimeinReverse) 1.0)
    (Variables|/Script/Engine.MovementComponent|SetVelocity (Variables|Default|GetProjectileMovement) (Math|Vector|MakeVector (* -1.2 (.X (Math|Vector|BreakVector (Variables|/Script/Engine.MovementComponent|GetVelocity (Variables|Default|GetProjectileMovement))))) (.Y (Math|Vector|BreakVector (Variables|/Script/Engine.MovementComponent|GetVelocity (Variables|Default|GetProjectileMovement)))) (.Z (Math|Vector|BreakVector (Variables|/Script/Engine.MovementComponent|GetVelocity (Variables|Default|GetProjectileMovement))))))
    (Development|PrintString "Hello")
    (Variables|Default|SetTimeinReverse 0.0)))

(fn WallBounce
  (params (Selection :type Integer))
  (bind _returnvalue (Math|Random|RandomFloatinRange -5e+01 5e+01))
  (switch int Selection
    (:-1
      (CallFunction|AddSpinWall (+ _returnvalue 125.0)))
    (:0
      (CallFunction|AddSpinWall (Math|Random|RandomFloatinRange -15.0 15.0)))
    (:1
      (CallFunction|AddSpinWall (+ _returnvalue -125.0))))
  (CallFunction|ReverseY))

(fn AddSpinWall
  (params (WallSpin :type Float%20%28single-precision%29))
  (Variables|/Script/Engine.MovementComponent|SetVelocity (Variables|Default|GetProjectileMovement) (+ (Math|Vector|MakeVector WallSpin 0.0 0.0) (Variables|/Script/Engine.MovementComponent|GetVelocity (Variables|Default|GetProjectileMovement)))))

(fn ReverseY
  (if (>= (Variables|Default|GetTimeinReverse) 1.0)
    (Variables|/Script/Engine.MovementComponent|SetVelocity (Variables|Default|GetProjectileMovement) (Math|Vector|MakeVector (.X (Math|Vector|BreakVector (Variables|/Script/Engine.MovementComponent|GetVelocity (Variables|Default|GetProjectileMovement)))) (* -1.0 (.Y (Math|Vector|BreakVector (Variables|/Script/Engine.MovementComponent|GetVelocity (Variables|Default|GetProjectileMovement))))) (.Z (Math|Vector|BreakVector (Variables|/Script/Engine.MovementComponent|GetVelocity (Variables|Default|GetProjectileMovement))))))
    (Development|PrintString "Hello")
    (Variables|Default|SetTimeinReverse 0.0)))